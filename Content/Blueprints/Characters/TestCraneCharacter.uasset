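; Test player crane character that moves sideways, flies up and down, rotates in quarter turns, and grabs and places physics blocks.
; Grab line-traces from CubePosition and constrains the hit body to the capsule; release breaks the constraint and calls SpawnBlockAfterBlock on a once-spawned Spawn_Block.
; Place Block cycles cube, rectangle and T-block, applying test-key rotations to the latter two and boosting mass after a delay.
; Camera-follow, animation and player-setup logic is disconnected.
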(event `Key|Zero`
  (params (Key :type "Key Structure"))
  ;[1 1 1] Add player 2
)

(event `InputAction|Grab`
  (params (Key :type "Key Structure"))
  (bind _cubeposition (`self.CubePosition`))
  (bind _returnvalue (`SceneComponent.K2_GetComponentLocation` _cubeposition))
  ;[1 0.2436 0.1739] Grab Crane Mechanic
  (:`Pressed`
    (bind (_outhit _returnvalue_2) (`KismetSystemLibrary.LineTraceSingle` :`Start` _returnvalue :`End` (+ _returnvalue (* (`SceneComponent.GetForwardVector` _cubeposition) (`KismetMathLibrary.Conv_DoubleToVector` 100.0))) :`TraceChannel` "TraceTypeQuery1" :`DrawDebugType` "ForDuration"))
    (if _returnvalue_2
      (bind (_bblockinghit _binitialoverlap _time _distance _location _impactpoint _normal _impactnormal _physmat _hitactor _hitcomponent) (`GameplayStatics.BreakHitResult` _outhit))
      (if (`SceneComponent.IsSimulatingPhysics` _hitcomponent "None")
        (`PhysicsHandleComponent.GrabComponentAtLocation` (`self.PhysicsHandle`) _hitcomponent "None" (`SceneComponent.K2_GetComponentLocation` _hitcomponent))
        (`PhysicsConstraintComponent.SetConstrainedComponents` (`self.PhysicsConstraint`) (`self.CapsuleComponent`) "None" _hitcomponent "None")
        (`PhysicsHandleComponent.ReleaseComponent` (`self.PhysicsHandle`)))))
  (:`Released`
    (`|ExecutionSequence`
      (:`then_0`
        (`/Engine/EditorBlueprintResources/StandardMacros.DoOnce` false
          (:`Completed`
            (bind _returnvalue_3 (`|SpawnActorFromClass` "/Game/Blueprints/Jamie/Spawn_Block.Spawn_Block_C" (`KismetMathLibrary.MakeTransform` (-442.748128 -442.748128 86.171578)) "Undefined" "MultiplyWithRoot" null null))
            (set `self.SpawnRef` _returnvalue_3))))
      (:`then_1`
        (`PhysicsConstraintComponent.BreakConstraint` (`self.PhysicsConstraint`))
        (bind _asspawn_block (cast `/Game/Blueprints/Jamie/Spawn_Block` (`self.SpawnRef`)))
        (`/Game/Blueprints/Jamie/Spawn_Block.Spawn Block after block` _asspawn_block)))))

(event `InputAxis|Left/Right`
  (params (AxisValue :type "Float (single-precision)"))
  ;[1 0.5084 0.03639] Movement Controls
  (`self.AddMovementInput` (1.0 0.0 0.0) AxisValue))

(event `InputAxis|Up/Down`
  (params (AxisValue :type "Float (single-precision)"))
  ;[1 1 1] Movement up and down
  (if (`NavMovementComponent.IsFlying` (`self.CharacterMovement`))
    (`self.AddMovementInput` (`self.GetActorUpVector` (`self.GetController`)) AxisValue)
    (`SceneComponent.K2_DetachFromComponent` (`self.Camera`) "KeepWorld" "KeepWorld" "KeepWorld" true)))

(event `self.ReceiveTick`
  (params (DeltaSeconds :type "Float (single-precision)"))
  ;[1 0.2436 0.1739] Grab Crane Mechanic
  (`PhysicsHandleComponent.SetTargetLocation` (`self.PhysicsHandle`) (`SceneComponent.K2_GetComponentLocation` (`self.CubePosition`))))

(event `UpdateControlRotation`
  ;[1 0.08921 0] Update Rotation of block when turning (Will change)
  (`/Engine/EditorBlueprintResources/StandardMacros.IsValid` (`self.GetController`)
    (:`Is Valid`
      (`/Engine/EditorBlueprintResources/StandardMacros.CompareFloat` (.x (`MovementComponent.Velocity` (`self.CharacterMovement`)))
        (:`>`
          (`Controller.SetControlRotation` (`self.GetController`) (`KismetMathLibrary.MakeRotator` 0.0)))
        (:`<`
          (`Controller.SetControlRotation` (`self.GetController`) (`KismetMathLibrary.MakeRotator` 0.0 0.0 180.0)))))))

(event `UpdateAnimation`
  ;[1 0.7403 0.1413] Update Animation when moving
  (`PaperFlipbookComponent.SetFlipbook` (`self.Sprite`) (select `bool` (> (`KismetMathLibrary.VSize` (`MovementComponent.Velocity` (`self.CharacterMovement`))) 0.0) :`false` "/Game/Blueprints/Sprites/Placeholder_assets_Sunnylandassets/PNG/sprites/player/idle/Player1Flipbook.Player1Flipbook" :`true` "/Game/Blueprints/Sprites/Placeholder_assets_Sunnylandassets/PNG/sprites/player/idle/Player1Flipbook.Player1Flipbook" :!type "PaperFlipbook Object Reference")))

(event `InputAction|Fly`
  (params (Key :type "Key Structure"))
  ;[1 0.3296 0.2838] Fly up and down
  (:`Pressed`
    (`CharacterMovementComponent.SetMovementMode` (`self.CharacterMovement`) "MOVE_Flying" 0)))

(event `InputAction|Rotate Right`
  (params (Key :type "Key Structure"))
  ;[1 0.2286 0.3264] Clockwise Rotate
  (:`Pressed`
    (`self.K2_SetActorRotation` (`KismetMathLibrary.MakeRotator` 0.0 (+ (`self.Rotate`) (`self.New Rotate`))))
    (if (`self.Rotated?`)
      (set `self.Rotate` 90.0)
      (set `self.Rotated?` false)
      (set `self.Rotated?2` true)
      (elif (`self.Rotated?2`)
        (set `self.Rotate` 180.0)
        (set `self.Rotated?2` false)
        (set `self.Rotated?3` true)
        (elif (`self.Rotated?3`)
          (set `self.Rotate` 270.0)
          (set `self.Rotated?3` false)
          (set `self.Rotated?4Reset` true)
          (elif (`self.Rotated?4Reset`)
            (set `self.Rotate` 0.0)
            (set `self.Rotated?4Reset` false)
            (set `self.Rotated?` true)))))))

(event `InputAction|Place Block`
  (params (Key :type "Key Structure"))
  (bind (_returnvalue_x _returnvalue_y _returnvalue_z) (`KismetMathLibrary.BreakVector` (`SceneComponent.K2_GetComponentLocation` (`Character.CapsuleComponent` (`GameplayStatics.GetPlayerCharacter` 0)))))
  (bind (_returnvalue_x_2 _returnvalue_y_2 _returnvalue_z_2) (`KismetMathLibrary.BreakVector` (`SceneComponent.K2_GetComponentLocation` (`Character.CapsuleComponent` (`GameplayStatics.GetPlayerCharacter` 0)))))
  (bind (_returnvalue_x_3 _returnvalue_y_3 _returnvalue_z_3) (`KismetMathLibrary.BreakVector` (`SceneComponent.K2_GetComponentLocation` (`Character.CapsuleComponent` (`GameplayStatics.GetPlayerCharacter` 0)))))
  (bind (_returnvalue_x_4 _returnvalue_y_4 _returnvalue_z_4) (`KismetMathLibrary.BreakVector` (`SceneComponent.K2_GetComponentLocation` (`Character.CapsuleComponent` (`GameplayStatics.GetPlayerCharacter` 0)))))
  ;[0.9614 1 0.2164] Spawn different blocks in order range
  (:`Pressed`
    (if (`self.Block 1`)
      ;;[0.02362 1 0] Cube Block
      (bind _returnvalue (`|SpawnActorFromClass` "/Game/Blueprints/Jamie/3DBlocks/3DCube_Block.3DCube_Block_C" (`KismetMathLibrary.MakeTransform` (`SceneComponent.K2_GetComponentLocation` (`Character.CapsuleComponent` (`GameplayStatics.GetPlayerCharacter` 0)))) "AdjustIfPossibleButAlwaysSpawn" "MultiplyWithRoot" null null))
      (set `self.Block 1` false)
      (set `self.Block 2` true)
      ;;[1 0.1879 0.5181] Make placed blocks heavier after a while
      (`KismetSystemLibrary.Delay` 1.0)
      (bind _as3dcube_block (cast `/Game/Blueprints/Jamie/3DBlocks/3DCube_Block` _returnvalue))
      (`PrimitiveComponent.SetMassScale` (`/Game/Blueprints/Jamie/3DBlocks/3DCube_Block.Cube` _as3dcube_block) "None" 100000.0)
      (`KismetSystemLibrary.Delay` 2.0)
      (elif (`self.Block 2`)
        ;;[1 0.212 0.01361] Rectangle Block
        (if (`self.RotateTest1`)
          (`|SpawnActorFromClass` "/Game/Blueprints/Jamie/3DBlocks/3DRectangle_Block.3DRectangle_Block_C" (`KismetMathLibrary.MakeTransform` (`SceneComponent.K2_GetComponentLocation` (`Character.CapsuleComponent` (`GameplayStatics.GetPlayerCharacter` 0))) (struct :`Pitch` 90.0)) "AdjustIfPossibleButAlwaysSpawn" "MultiplyWithRoot" null null)
          (set `self.Block 2` false)
          (set `self.Block 3` true)
          ;;;[1 0.2099 0.5232] Make blocks heavier after delay
          (`KismetSystemLibrary.Delay` 1.0)
          (bind _as3drectangle_block (cast `/Game/Blueprints/Jamie/3DBlocks/3DRectangle_Block` null))
          (`PrimitiveComponent.SetMassScale` (`/Game/Blueprints/Jamie/3DBlocks/3DRectangle_Block.Cube` _as3drectangle_block) "None" 100000.0)
          (else
            (bind _returnvalue_2 (`|SpawnActorFromClass` "/Game/Blueprints/Jamie/3DBlocks/3DRectangle_Block.3DRectangle_Block_C" (`KismetMathLibrary.MakeTransform` (`SceneComponent.K2_GetComponentLocation` (`Character.CapsuleComponent` (`GameplayStatics.GetPlayerCharacter` 0)))) "AdjustIfPossibleButAlwaysSpawn" "MultiplyWithRoot" null null))
            (set `self.Block 2` false)
            (set `self.Block 3` true)
            ;;;[1 0.2099 0.5232] Make blocks heavier after delay
            (`KismetSystemLibrary.Delay` 1.0)
            (bind _as3drectangle_block_2 (cast `/Game/Blueprints/Jamie/3DBlocks/3DRectangle_Block` _returnvalue_2))
            (`PrimitiveComponent.SetMassScale` (`/Game/Blueprints/Jamie/3DBlocks/3DRectangle_Block.Cube` _as3drectangle_block_2) "None" 100000.0)))
        (elif (`self.Block 3`)
          ;;[0.1881 0.2496 1] T-Block
          (if (`self.RotateTest1`)
            ;;;[0.0643 1 0.9781] 90 Rotate
            (bind _returnvalue_3 (`|SpawnActorFromClass` "/Game/Blueprints/Jamie/3DBlocks/3DT_Block.3DT_Block_C" (`KismetMathLibrary.MakeTransform` (`KismetMathLibrary.MakeVector` _returnvalue_x_3 _returnvalue_y_3 _returnvalue_z_3) (struct :`Pitch` 90.0)) "AdjustIfPossibleButAlwaysSpawn" "MultiplyWithRoot" null null))
            (set `self.Block 3` false)
            (set `self.Block 1` true)
            ;;;[1 0.3104 0.8135] Make blocks heavier after delay
            (`KismetSystemLibrary.Delay` 1.0)
            (bind _as3dt_block (cast `/Game/Blueprints/Jamie/3DBlocks/3DT_Block` _returnvalue_3))
            (`PrimitiveComponent.SetMassScale` (`/Game/Blueprints/Jamie/3DBlocks/3DT_Block.Cube` _as3dt_block) "None" 100000.0)
            (elif (`self.RotateTest2`)
              ;;;[0.1435 0.7306 1] 180 Rotate
              (bind _returnvalue_4 (`|SpawnActorFromClass` "/Game/Blueprints/Jamie/3DBlocks/3DT_Block.3DT_Block_C" (`KismetMathLibrary.MakeTransform` (`KismetMathLibrary.MakeVector` _returnvalue_x_4 _returnvalue_y_4 _returnvalue_z_4) (struct :`Pitch` 180.0)) "AdjustIfPossibleButAlwaysSpawn" "MultiplyWithRoot" null null))
              (set `self.Block 3` false)
              (set `self.Block 1` true)
              ;;;[1 0.3104 0.8135] Make blocks heavier after delay
              (`KismetSystemLibrary.Delay` 1.0)
              (bind _as3dt_block_2 (cast `/Game/Blueprints/Jamie/3DBlocks/3DT_Block` _returnvalue_4))
              (`PrimitiveComponent.SetMassScale` (`/Game/Blueprints/Jamie/3DBlocks/3DT_Block.Cube` _as3dt_block_2) "None" 100000.0)
              (elif (`self.RotateTest3`)
                ;;;[0.2421 0.9102 1] 270 Rotate
                (bind _returnvalue_5 (`|SpawnActorFromClass` "/Game/Blueprints/Jamie/3DBlocks/3DT_Block.3DT_Block_C" (`KismetMathLibrary.MakeTransform` (`KismetMathLibrary.MakeVector` _returnvalue_x _returnvalue_y _returnvalue_z) (struct :`Pitch` 270.0)) "AdjustIfPossibleButAlwaysSpawn" "MultiplyWithRoot" null null))
                (set `self.Block 3` false)
                (set `self.Block 1` true)
                ;;;[1 0.3104 0.8135] Make blocks heavier after delay
                (`KismetSystemLibrary.Delay` 1.0)
                (bind _as3dt_block_3 (cast `/Game/Blueprints/Jamie/3DBlocks/3DT_Block` _returnvalue_5))
                (`PrimitiveComponent.SetMassScale` (`/Game/Blueprints/Jamie/3DBlocks/3DT_Block.Cube` _as3dt_block_3) "None" 100000.0)
                (else
                  ;;;[1 1 1] No Rotate
                  (bind _returnvalue_6 (`|SpawnActorFromClass` "/Game/Blueprints/Jamie/3DBlocks/3DT_Block.3DT_Block_C" (`KismetMathLibrary.MakeTransform` (`KismetMathLibrary.MakeVector` _returnvalue_x_2 _returnvalue_y_2 _returnvalue_z_2)) "AdjustIfPossibleButAlwaysSpawn" "MultiplyWithRoot" null null))
                  (set `self.Block 3` false)
                  (set `self.Block 1` true)
                  ;;;[1 0.3104 0.8135] Make blocks heavier after delay
                  (`KismetSystemLibrary.Delay` 1.0)
                  (bind _as3dt_block_4 (cast `/Game/Blueprints/Jamie/3DBlocks/3DT_Block` _returnvalue_6))
                  (`PrimitiveComponent.SetMassScale` (`/Game/Blueprints/Jamie/3DBlocks/3DT_Block.Cube` _as3dt_block_4) "None" 100000.0))))))))))

(event `InputAction|Rotate Left`
  (params (Key :type "Key Structure"))
  ;[1 0.4922 0.1414] Anticlcokwise Rotate
  (:`Pressed`
    (`self.K2_SetActorRotation` (`KismetMathLibrary.MakeRotator` 0.0 (- (`self.AnticlockwiseRotate`) (`self.New Rotate`))))
    (if (`self.Rotated?`)
      (set `self.AnticlockwiseRotate` 270.0)
      (set `self.Rotated?` false)
      (set `self.Rotated?2` true)
      (elif (`self.Rotated?2`)
        (set `self.AnticlockwiseRotate` 180.0)
        (set `self.Rotated?2` false)
        (set `self.Rotated?3` true)
        (elif (`self.Rotated?3`)
          (set `self.AnticlockwiseRotate` 90.0)
          (set `self.Rotated?3` false)
          (set `self.Rotated?4Reset` true)
          (elif (`self.Rotated?4Reset`)
            (set `self.AnticlockwiseRotate` 360.0)
            (set `self.Rotated?4Reset` false)
            (set `self.Rotated?` true)))))))

(event `InputAction|RotationTest1`
  (params (Key :type "Key Structure"))
  ;[0.09641 0.9502 1] Rotate
  (:`Pressed`
    (set `self.RotateTest1` true)
    (set `self.RotateTest2` false)
    (set `self.RotateTest3` false)))

(event `InputAction|RotationTest2`
  (params (Key :type "Key Structure"))
  ;[0.09641 0.9502 1] Rotate
  (:`Pressed`
    (set `self.RotateTest2` true)
    (set `self.RotateTest3` false)
    (set `self.RotateTest1` false)))

(event `InputAction|RotationTest3`
  (params (Key :type "Key Structure"))
  ;[0.09641 0.9502 1] Rotate
  (:`Pressed`
    (set `self.RotateTest3` true)
    (set `self.RotateTest1` false)
    (set `self.RotateTest2` false)))

(event `InputAction|RotationTest4`
  (params (Key :type "Key Structure"))
  ;[0.09641 0.9502 1] Rotate
  (:`Pressed`
    (set `self.RotateTest1` false)
    (set `self.RotateTest2` false)
    (set `self.RotateTest3` false)))

(fn `SpawnFunc`)

(fn `UserConstructionScript`)