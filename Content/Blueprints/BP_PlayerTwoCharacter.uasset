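; Player two's Paper2D side-scroller character, with left/right movement, flying and block placement.
; Tick updates the flipbook (both states use Player1Flipbook) and turns the controller yaw by X velocity.
; Fly switches to Flying mode, where Up/Down moves vertically and detaches the camera.
; Place Block spawns a Cube_Block at player index 0's capsule; the spline camera follow is unconnected, though BeginPlay caches its actor.
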(event `self.ReceiveBeginPlay`
  (bind _returnvalue (`GameplayStatics.GetActorOfClass` "/Game/Camera/Bp_Camreaspline2.Bp_Camreaspline2_C"))
  (set `self.CameraRef2` _returnvalue))

(event `self.ReceiveTick`
  (params (DeltaSeconds :type "Float (single-precision)"))
  ;[0 1 0.1855] Event Tick
  (`self.UpdateAnimation`)
  (`self.UpdateControlRotation`))

(event `InputAxis|MoveRight`
  (params (AxisValue :type "Float (single-precision)"))
  ;[1 0.5084 0.03639] Movement Controls
  (`self.AddMovementInput` (1.0 0.0 0.0) AxisValue))

(event `InputAxis|Up/Down`
  (params (AxisValue :type "Float (single-precision)"))
  (if (`NavMovementComponent.IsFlying` (`self.CharacterMovement`))
    (`self.AddMovementInput` (`self.GetActorUpVector` (`self.GetController`)) AxisValue)
    (`SceneComponent.K2_DetachFromComponent` (`self.Camera`) "KeepWorld" "KeepWorld" "KeepWorld" true)))

(event `InputAction|Fly`
  (params (Key :type "Key Structure"))
  (:`Pressed`
    (`CharacterMovementComponent.SetMovementMode` (`self.CharacterMovement`) "MOVE_Flying" 0)))

(event `UpdateAnimation`
  ;[1 0.7403 0.1413] Update Animation when moving
  (`PaperFlipbookComponent.SetFlipbook` (`self.Sprite`) (select `bool` (> (`KismetMathLibrary.VSize` (`MovementComponent.Velocity` (`self.CharacterMovement`))) 0.0) :`false` "/Game/Blueprints/Sprites/Placeholder_assets_Sunnylandassets/PNG/sprites/player/idle/Player1Flipbook.Player1Flipbook" :`true` "/Game/Blueprints/Sprites/Placeholder_assets_Sunnylandassets/PNG/sprites/player/idle/Player1Flipbook.Player1Flipbook" :!type "PaperFlipbook Object Reference")))

(event `UpdateControlRotation`
  ;[1 0.08921 0] Update Rotation of block when turning (Will change)
  (`/Engine/EditorBlueprintResources/StandardMacros.IsValid` (`self.GetController`)
    (:`Is Valid`
      (`/Engine/EditorBlueprintResources/StandardMacros.CompareFloat` (.x (`MovementComponent.Velocity` (`self.CharacterMovement`)))
        (:`>`
          (`Controller.SetControlRotation` (`self.GetController`) (`KismetMathLibrary.MakeRotator` 0.0)))
        (:`<`
          (`Controller.SetControlRotation` (`self.GetController`) (`KismetMathLibrary.MakeRotator` 0.0 0.0 180.0)))))))

(event `InputAction|Place Block`
  (params (Key :type "Key Structure"))
  (:`Pressed`
    (`|SpawnActorFromClass` "/Game/Blueprints/Jamie/Blocks/Cube_Block.Cube_Block_C" (`KismetMathLibrary.MakeTransform` (`SceneComponent.K2_GetComponentLocation` (`Character.CapsuleComponent` (`GameplayStatics.GetPlayerCharacter` 0)))) "AdjustIfPossibleButAlwaysSpawn" "MultiplyWithRoot" null null)))

(fn `UserConstructionScript`)