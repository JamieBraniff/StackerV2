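; GM_PlayerOne is a game mode scaffold for local multiplayer, with most of its logic disconnected.
; BeginPlay, the player 2 events, SpawnInputReceivers and SpawnPlayer are empty.
; GetPlayerStartPoints caches PlayerStarts, but its only call is unwired.
; Unwired nodes sketch adding or removing player 2, creating possessed Input_Receivers at starts ordered by numeric tag, and spawning BP_PlayerOneCharacter at a receiver.
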(event `DestroyPlayer2`
  ;[1 1 1] Robbie's players
)

(event `SpawnPlayer2`
  ;[1 1 1] Robbie's players
)

(event `AdjustPlayers`
  ;[1 1 1] Robbie's players
)

(event `self.ReceiveBeginPlay`)

(fn `GetPlayerStartPoints`
  (bind _outactors (`GameplayStatics.GetAllActorsOfClass` "/Script/Engine.PlayerStart"))
  (set `self.PlayerStartArray` _outactors))

(fn `NameToInt`
  (params (PlayerStart :type "PlayerStart Object Reference"))
  (returns (ReturnValue :type Integer))
  (return (`KismetStringLibrary.Conv_StringToInt` (`KismetStringLibrary.Conv_NameToString` (`PlayerStart.PlayerStartTag` PlayerStart)))))

(fn `SpawnInputReceivers`
  ;[1 0.2193 0.4063] Making a list of player spawns for the player to control from start
)

(fn `SpawnPlayer`
  (params (CurrentPlayerIndex :type Integer) (`Input Receiver` :type "/Game/Blueprints/Jamie/Multiplayer/Input_Receiver Object Reference"))
  (returns (Return :type Boolean))
  ;[0.3259 1 0.2274] Spawns player character where input receiver is
)

(fn `SpawnPlayerF`
  (returns (Return :type Boolean))
  (return false))

(fn `UserConstructionScript`)