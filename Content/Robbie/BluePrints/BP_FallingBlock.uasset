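; Falling Tetris-style piece that steps down the playfield until it lands.
; The construction script picks one of seven shapes at random by offsetting four cubes and tints their material glow to match.
; A looping timer line-traces below each cube against WorldStatic, moving the actor down one cell when clear.
; On a hit it stops, replaces each cube with a coloured BP_SingleBlock, spawns the next falling block and destroys itself.
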(event `self.ReceiveBeginPlay`
  ;[1 1 1] Block Fall/Land
  (bind _returnvalue (`KismetSystemLibrary.K2_SetTimerDelegate` (delegate `DropBlock`) (`self.DropSpeed`) true))
  (set `self.BlockDroppingTimer` _returnvalue))

(event `DropBlock`
  ;[1 1 1] Block Fall/Land
  (set `self.ShouldDrop?` true)
  (for _array_element (`SceneComponent.GetChildrenComponents` (`self.DefaultSceneRoot`) false)
    (bind _returnvalue (`SceneComponent.K2_GetComponentLocation` _array_element))
    (bind (_outhit _returnvalue_2) (`KismetSystemLibrary.LineTraceSingleForObjects` _returnvalue (- _returnvalue (0.0 0.0 50.0)) (`|MakeArray` "ObjectTypeQuery1" :!type "EObjectTypeQuery Enum")))
    (if _returnvalue_2
      (`/Engine/EditorBlueprintResources/StandardMacros.DoOnce` false
        (:`Completed`
          (set `self.ShouldDrop?` false)
          (`KismetSystemLibrary.K2_ClearAndInvalidateTimerHandle` (`self.BlockDroppingTimer`))))))
  ;[1 1 1] Once Block No Longer Falling,Swap to single Blocks and spawn New
  (if (`self.ShouldDrop?`)
    (`self.K2_AddActorLocalOffset` (0.0 0.0 -50.0))
    (else
      (for _array_element_2 (`SceneComponent.GetChildrenComponents` (`self.DefaultSceneRoot`) false)
        (`|SpawnActorFromClass` "/Game/Robbie/BluePrints/BP_SingleBlock.BP_SingleBlock_C" (`KismetMathLibrary.MakeTransform` (`SceneComponent.K2_GetComponentLocation` _array_element_2)) "Undefined" "MultiplyWithRoot" null (`self.BlockColour`) null))
      (`|SpawnActorFromClass` "BP_FallingBlock_C" (`KismetMathLibrary.MakeTransform` (0.0 -0.0 1000.0)) "Undefined" "MultiplyWithRoot" null null)
      (`self.K2_DestroyActor`))))

(fn `UserConstructionScript`
  (switch `int` (`KismetMathLibrary.RandomIntegerInRange` 0 6)
    (:`0`
      ;[1 1 1] Make Line Block
      (`SceneComponent.K2_AddLocalOffset` (`self.Cube2`) (0.0 0.0 50.0) false false)
      (`SceneComponent.K2_AddLocalOffset` (`self.Cube3`) (0.0 0.0 100.0) false false)
      (`SceneComponent.K2_AddLocalOffset` (`self.Cube4`) (0.0 0.0 150.0) false false)
      (set `self.BlockColour` (struct :`R` 1.0 :`G` 0.977855 :`A` 1.0)))
    (:`1`
      ;[1 1 1] Make L Block
      (`SceneComponent.K2_AddLocalOffset` (`self.Cube2`) (0.0 0.0 50.0) false false)
      (`SceneComponent.K2_AddLocalOffset` (`self.Cube3`) (0.0 0.0 100.0) false false)
      (`SceneComponent.K2_AddLocalOffset` (`self.Cube4`) (0.0 50.0 0.0) false false)
      (set `self.BlockColour` (struct :`R` 1.0 :`G` 0.053491 :`A` 1.0)))
    (:`2`
      ;[1 1 1] Make Backwards L Block
      (`SceneComponent.K2_AddLocalOffset` (`self.Cube2`) (0.0 0.0 50.0) false false)
      (`SceneComponent.K2_AddLocalOffset` (`self.Cube3`) (0.0 0.0 100.0) false false)
      (`SceneComponent.K2_AddLocalOffset` (`self.Cube4`) (0.0 -50.0 0.0) false false)
      (set `self.BlockColour` (struct :`R` 1.0 :`G` 0.490642 :`A` 1.0)))
    (:`3`
      ;[1 1 1] Make S Block
      (`SceneComponent.K2_AddLocalOffset` (`self.Cube2`) (0.0 0.0 50.0) false false)
      (`SceneComponent.K2_AddLocalOffset` (`self.Cube3`) (0.0 50.0 50.0) false false)
      (`SceneComponent.K2_AddLocalOffset` (`self.Cube4`) (0.0 50.0 100.0) false false)
      (set `self.BlockColour` (struct :`R` 1.0 :`B` 0.776372 :`A` 1.0)))
    (:`4`
      ;[1 1 1] Make Backwards S Block
      (`SceneComponent.K2_AddLocalOffset` (`self.Cube2`) (0.0 0.0 50.0) false false)
      (`SceneComponent.K2_AddLocalOffset` (`self.Cube3`) (0.0 -50.0 50.0) false false)
      (`SceneComponent.K2_AddLocalOffset` (`self.Cube4`) (0.0 -50.0 100.0) false false)
      (set `self.BlockColour` (struct :`R` 0.277469 :`B` 0.421875 :`A` 1.0)))
    (:`5`
      ;[1 1 1] Make T Block
      (`SceneComponent.K2_AddLocalOffset` (`self.Cube2`) (0.0 -50.0 0.0) false false)
      (`SceneComponent.K2_AddLocalOffset` (`self.Cube3`) (0.0 50.0 0.0) false false)
      (`SceneComponent.K2_AddLocalOffset` (`self.Cube4`) (0.0 0.0 50.0) false false)
      (set `self.BlockColour` (struct :`G` 0.97504 :`B` 1.0 :`A` 1.0)))
    (:`6`
      ;[1 1 1] Make Square Block
      (`SceneComponent.K2_AddLocalOffset` (`self.Cube2`) (0.0 0.0 50.0) false false)
      (`SceneComponent.K2_AddLocalOffset` (`self.Cube3`) (0.0 50.0 0.0) false false)
      (`SceneComponent.K2_AddLocalOffset` (`self.Cube4`) (0.0 50.0 50.0) false false)
      (set `self.BlockColour` (struct :`R` 0.070988 :`G` 1.0 :`A` 1.0))))
  ;[1 1 1] Colour Takes Affect
  (`MeshComponent.SetVectorParameterValueOnMaterials` (`self.Cube1`) "GlowColor" (`KismetMathLibrary.Conv_LinearColorToVector` (`self.BlockColour`)))
  (`MeshComponent.SetVectorParameterValueOnMaterials` (`self.Cube2`) "GlowColor" (`KismetMathLibrary.Conv_LinearColorToVector` (`self.BlockColour`)))
  (`MeshComponent.SetVectorParameterValueOnMaterials` (`self.Cube3`) "GlowColor" (`KismetMathLibrary.Conv_LinearColorToVector` (`self.BlockColour`)))
  (`MeshComponent.SetVectorParameterValueOnMaterials` (`self.Cube4`) "GlowColor" (`KismetMathLibrary.Conv_LinearColorToVector` (`self.BlockColour`))))