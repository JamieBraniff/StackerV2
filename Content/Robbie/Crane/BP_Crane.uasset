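; BP_Crane is a player-controlled crane that moves its Base sideways and vertically through Enhanced Input and picks up objects below it.
; Holding Space line-traces downward and grabs the hit component with a PhysicsHandle, releasing it on key up.
; Tick keeps the held object's target at the trace's far end below Base.
; Tick also eases the camera toward the closest point to the actor on a BP_CameraSplineRL spline.
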(event `self.ReceiveBeginPlay`
  ;[1 1 1] Adding Controlls
  (`|ExecutionSequence`
    (:`then_0`
      ;[1 0.3529 0.3529] CameraSpline
      (bind _returnvalue (`GameplayStatics.GetActorOfClass` "/Game/Robbie/CameraSpline/BP_CameraSplineRL.BP_CameraSplineRL_C"))
      (set `self.CameraSplineREF` _returnvalue))
    (:`then_1`
      (bind _asplayer_controller (cast `PlayerController` (`self.GetController`)))
      (bind _returnvalue_2 (pcsubsystem `EnhancedInputLocalPlayerSubsystem` _asplayer_controller))
      (`/Engine/EditorBlueprintResources/StandardMacros.IsValid` _returnvalue_2
        (:`Is Valid`
          (`EnhancedInputSubsystemInterface.AddMappingContext` _returnvalue_2 "/Game/Robbie/Inputs/CraneMapping.CraneMapping" 0 (struct)))))))

(event `EnhancedInput|/Game/Robbie/Inputs/MoveRightLeft_IA`
  (params (ActionValue :type "Float (double-precision)") (ElapsedSeconds :type "Float (double-precision)") (TriggeredSeconds :type "Float (double-precision)") (InputAction :type "InputAction Object Reference" :default "/Game/Robbie/Inputs/MoveRightLeft_IA.MoveRightLeft_IA"))
  ;[1 1 1] Movements
  (:`Triggered`
    (`SceneComponent.K2_AddLocalOffset` (`self.Base`) (`KismetMathLibrary.MakeVector` 0.0 (* ActionValue (`self.PlayerSpeed`))) false false)))

(event `Key|SpaceBar`
  (params (Key :type "Key Structure"))
  (bind _base (`self.Base`))
  (bind _returnvalue (`SceneComponent.K2_GetComponentLocation` _base))
  ;[1 1 1] Grab
  (:`Pressed`
    (bind (_outhit _returnvalue_2) (`KismetSystemLibrary.LineTraceSingle` :`Start` _returnvalue :`End` (+ _returnvalue (* (`KismetMathLibrary.NegateVector` (`KismetMathLibrary.GetUpVector` (`SceneComponent.K2_GetComponentRotation` _base))) 1000.0)) :`TraceChannel` "TraceTypeQuery1" :`DrawDebugType` "Persistent"))
    (if _returnvalue_2
      (bind (_bblockinghit _binitialoverlap _time _distance _location _impactpoint _normal _impactnormal _physmat _hitactor _hitcomponent) (`GameplayStatics.BreakHitResult` _outhit))
      (`PhysicsHandleComponent.GrabComponentAtLocationWithRotation` :`self` (`self.PhysicsHandle`) :`Component` _hitcomponent :`Location` (`SceneComponent.K2_GetComponentLocation` _hitcomponent))
      (set `self.IsGrabbingObject?` true)))
  (:`Released`
    (if (`self.IsGrabbingObject?`)
      (`PhysicsHandleComponent.ReleaseComponent` (`self.PhysicsHandle`))
      (set `self.IsGrabbingObject?` false))))

(event `EnhancedInput|/Game/Robbie/Inputs/MoveUpDown_IA`
  (params (ActionValue :type "Float (double-precision)") (ElapsedSeconds :type "Float (double-precision)") (TriggeredSeconds :type "Float (double-precision)") (InputAction :type "InputAction Object Reference" :default "/Game/Robbie/Inputs/MoveUpDown_IA.MoveUpDown_IA"))
  ;[1 1 1] Movements
  (:`Triggered`
    (`SceneComponent.K2_AddLocalOffset` (`self.Base`) (`KismetMathLibrary.MakeVector` 0.0 0.0 (* ActionValue (`self.PlayerSpeed`))) false false)))

(event `self.ReceiveTick`
  (params (DeltaSeconds :type "Float (single-precision)"))
  (bind _base (`self.Base`))
  ;[1 1 1] Pick up Loop
  (`|ExecutionSequence`
    (:`then_0`
      ;[1 0.3529 0.3529] Moving Camera
      (`SceneComponent.K2_SetWorldLocation` (`self.Camera`) (`KismetMathLibrary.VInterpTo` (`SceneComponent.K2_GetComponentLocation` (`self.Camera`)) (`SplineComponent.FindLocationClosestToWorldLocation` (`/Game/Robbie/CameraSpline/BP_CameraSplineRL.Spline` (`self.CameraSplineREF`)) (`self.K2_GetActorLocation`) "World") (`GameplayStatics.GetWorldDeltaSeconds`) 2.0) false false))
    (:`then_1`
      (if (`self.IsGrabbingObject?`)
        (`PhysicsHandleComponent.SetTargetLocation` (`self.PhysicsHandle`) (+ (`SceneComponent.K2_GetComponentLocation` _base) (* (`KismetMathLibrary.NegateVector` (`KismetMathLibrary.GetUpVector` (`SceneComponent.K2_GetComponentRotation` _base))) 1000.0)))))))

(fn `UserConstructionScript`)